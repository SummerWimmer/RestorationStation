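; Item data component that turns its owning actor into a pickup for the inventory system.
; On BeginPlay it sets the owner to replicate.
; Interactwith passes the item row name and quantity to the interacting player's InventorySystem, then destroys the owner if the add succeeds.
; LookAt returns an empty string.
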(event `self.ReceiveBeginPlay`
  (`Actor.SetReplicates` (`self.GetOwner`) true))

(event `/Game/Blueprints/Inventory/BPI_InteractInterface.InteractWith`
  (params (PlayerC :type "/Game/FirstPerson/Blueprints/BP_FirstPersonCharacter Object Reference"))
  (bind (_inventorysystem _inventorysystem_2) (`/Game/FirstPerson/Blueprints/BP_FirstPersonCharacter.InventorySystem` PlayerC))
  (bind (_itemid_datatable _itemid_rowname) (break `DataTableRowHandle` (`self.ItemID`)))
  (`/Engine/EditorBlueprintResources/StandardMacros.IsValid` _inventorysystem_2
    (:`Is Valid`
      (bind _seccess (`/Game/Blueprints/Inventory/InventorySystem.AddToInv` _inventorysystem_2 _itemid_rowname (`self.Quantity`)))
      (if _seccess
        (`Actor.K2_DestroyActor` (`self.GetOwner`))))))

(fn `LookAt`
  (returns (Message :type Text))
  (return ""))