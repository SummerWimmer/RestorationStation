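; Player Blueprint that sets up Enhanced Input and the HUD, and handles interaction and pausing.
; IA_Interact messages a valid LookAtActor, though nothing here sets that variable.
; P opens a pause menu with cursor and UI-only input outside MainMenu.
; Each tick, a forward line trace one TileSize long converts Paper2D tile map hits to tile coordinates and prints the tile index as debug output.
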(event `self.ReceiveBeginPlay`
  (`|ExecutionSequence`
    (:`then_0`
      (bind _asrs_player_controller (cast `/Game/Player/RS_PlayerController` (`self.GetController`)))
      (`EnhancedInputSubsystemInterface.AddMappingContext` (pcsubsystem `EnhancedInputLocalPlayerSubsystem` _asrs_player_controller) "/Game/Player/Input/IMC_Default.IMC_Default" 0 (struct)))
    (:`then_1`
      (bind _returnvalue (`|CreateWidget` "/Game/Widgets/W_Hud.W_Hud_C" (`GameplayStatics.GetPlayerController` 0)))
      (bind _output_get (set `self.Hud` _returnvalue))
      (`UserWidget.AddToViewport` _output_get 0))))

(event `self.ReceiveTick`
  (params (DeltaSeconds :type "Float (single-precision)"))
  (`self.Check Look At`))

(event `EnhancedInput|/Game/Player/Input/Actions/IA_Interact`
  (params (ActionValue :type Boolean) (ElapsedSeconds :type "Float (double-precision)") (TriggeredSeconds :type "Float (double-precision)") (InputAction :type "InputAction Object Reference" :default "/Game/Player/Input/Actions/IA_Interact.IA_Interact"))
  (bind _lookatactor (`self.LookAtActor`))
  (:`Started`
    (`/Engine/EditorBlueprintResources/StandardMacros.IsValid` _lookatactor
      (:`Is Valid`
        (message `/Game/Blueprints/Inventory/BPI_InteractInterface.InteractWith` _lookatactor self)))))

(event `EnhancedInput|/Game/Player/Input/Actions/IA_HideHeld`
  (params (ActionValue :type Boolean) (ElapsedSeconds :type "Float (double-precision)") (TriggeredSeconds :type "Float (double-precision)") (InputAction :type "InputAction Object Reference" :default "/Game/Player/Input/Actions/IA_HideHeld.IA_HideHeld")))

(event `Key|P`
  (params (Key :type "Key Structure"))
  (bind _returnvalue (`GameplayStatics.GetPlayerController` 0))
  ; Pause Menu - What level are we on?
  (:`Pressed`
    (bind _returnvalue_2 (`GameplayStatics.GetCurrentLevelName` true))
    ; Are we on Main Menu?
    (if (not (`KismetStringLibrary.EqualEqual_StrStr` "MainMenu" _returnvalue_2))
      ; Create/View Pause menu with Cursor
      (bind _returnvalue_3 (`|CreateWidget` "/Game/Widgets/PauseMenu.PauseMenu_C")) ; NO
      (set `PlayerController.bShowMouseCursor` true _returnvalue)
      (`WidgetBlueprintLibrary.SetInputMode_UIOnlyEx` _returnvalue _returnvalue_3 "LockAlways")
      (`UserWidget.AddToPlayerScreen` _returnvalue_3 0))))

(fn `Check Look At`
  (locals (TileX :type "Float (double-precision)") (TileY :type "Float (double-precision)"))
  (bind _returnvalue (`self.K2_GetActorLocation`))
  (bind _outhit (`KismetSystemLibrary.LineTraceSingle` :`Start` _returnvalue :`End` (+ _returnvalue (* (`self.GetActorForwardVector`) (`self.TileSize`))) :`TraceChannel` "TraceTypeQuery1" :`DrawDebugType` "ForOneFrame"))
  (bind (_bblockinghit _binitialoverlap _time _distance _location _impactpoint _normal _impactnormal _physmat _hitactor) (`GameplayStatics.BreakHitResult` _outhit))
  (bind _aspaper_tile_map_actor (cast `PaperTileMapActor` _hitactor))
  (bind (_returnvalue_x _returnvalue_y) (`KismetMathLibrary.BreakVector` (`self.K2_GetActorLocation` _aspaper_tile_map_actor)))
  (bind _rendercomponent (`PaperTileMapActor.RenderComponent` _aspaper_tile_map_actor))
  (bind _tilemap (`PaperTileMapComponent.TileMap` _rendercomponent))
  (bind _output_get (set `local.TileX` (/ (- (.x _location) _returnvalue_x) (`PaperTileMap.TileHeight` _tilemap))))
  (bind _output_get_2 (set `local.TileY` (/ (- (.y _location) _returnvalue_y) (`PaperTileMap.TileWidth` _tilemap))))
  (`KismetSystemLibrary.PrintString` (`KismetStringLibrary.Conv_IntToString` (`TileMapBlueprintLibrary.BreakTile` (`PaperTileMapComponent.GetTile` _rendercomponent (`KismetMathLibrary.FTrunc` _output_get) (`KismetMathLibrary.FTrunc` _output_get_2) 0)))))

(fn `LookAt`
  (returns (Message :type Text))
  (return ""))

(fn `UserConstructionScript`)