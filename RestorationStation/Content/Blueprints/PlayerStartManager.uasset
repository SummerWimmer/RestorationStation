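; PlayerStartManager is a level-transition trigger that moves the player to another level at a chosen player start.
; On BeginPlay it plays a FadeToDarkness widget in reverse to fade the screen in.
; When the player pawn overlaps its box, it plays the fade, waits briefly, stores its start tag in the GI_Main game instance and opens the named level.
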(event `self.ReceiveBeginPlay`
  (bind _returnvalue (`|CreateWidget` "/Game/Widgets/FadeToDarkness.FadeToDarkness_C"))
  (`UserWidget.AddToViewport` _returnvalue 0)
  (`/Game/Widgets/FadeToDarkness.playReverse` _returnvalue))

(event `self.Box.OnComponentBeginOverlap`
  (params (OverlappedComponent :type "PrimitiveComponent Object Reference") (OtherActor :type "Actor Object Reference") (OtherComp :type "PrimitiveComponent Object Reference") (OtherBodyIndex :type Integer) (bFromSweep :type Boolean) (SweepResult :type "HitResult Structure (by ref)"))
  ; Player Start Spawn Manager
  (if (== OtherActor (`GameplayStatics.GetPlayerPawn` 0))
    ;[0.15 0.05468 0.05617 0.5] Fade To Black Transition
    (bind _returnvalue (`|CreateWidget` "/Game/Widgets/FadeToDarkness.FadeToDarkness_C"))
    (`UserWidget.AddToViewport` _returnvalue 0)
    (`/Game/Widgets/FadeToDarkness.playFade` _returnvalue)
    (`KismetSystemLibrary.Delay` 1.2)
    (bind _asgi_main (cast `/Game/GI_Main` (`GameplayStatics.GetGameInstance`)))
    (set `/Game/GI_Main.Start Tag` (`self.S Tag`) _asgi_main)
    (`GameplayStatics.OpenLevel` (`self.Level Name`))))

(fn `UserConstructionScript`)