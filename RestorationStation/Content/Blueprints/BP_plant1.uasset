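; BP_plant1 is a Paper2D crop plant that grows through five sprite stages over time.
; From BeginPlay, a self-looping one-second Delay stands in for Tick and runs until PlantCycle exceeds MaxGrowth.
; Each pass rolls a one-in-five chance to set the sprite selected by PlantCycle, then increment that counter.
; Debug print nodes for growth are left disconnected.
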(event `self.ReceiveBeginPlay`
  ; Plant growth cycle
  (if (<= (`self.PlantCycle`) (`self.MaxGrowth`)) :!label _label
    (`KismetSystemLibrary.Delay` 1.0) ; tick speed
    (if (== (`KismetMathLibrary.RandomInteger` 5) 1)
      ;; Select and set plant image/ growth
      (`PaperSpriteComponent.SetSprite` (`self.PaperSprite`) (select `int` (`self.PlantCycle`) :`0` "/Game/Tilesets/Farm/farmsprites/farm_Sprite_110.farm_Sprite_110" :`1` "/Game/Tilesets/Farm/farmsprites/farm_Sprite_111.farm_Sprite_111" :`2` "/Game/Tilesets/Farm/farmsprites/farm_Sprite_112.farm_Sprite_112" :`3` "/Game/Tilesets/Farm/farmsprites/farm_Sprite_113.farm_Sprite_113" :`4` "/Game/Tilesets/Farm/farmsprites/farm_Sprite_114.farm_Sprite_114" :!type "PaperSprite Object Reference"))
      (bind _result (`/Engine/EditorBlueprintResources/StandardMacros.IncrementInt` (`self.PlantCycle`)) ; increase growth count
        (:`  `
          (goto _label)))
      (else
        (goto _label)))))

(fn `UserConstructionScript`)