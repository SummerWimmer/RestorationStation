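; BP_LootBag is an interactable loot container that exposes its InventorySystem to the player.
; Interactwith opens that inventory in the HUD of player 0's RS_PlayerController, and an inventory update that leaves it empty hides the container panel.
; LookAt returns an empty string.
; Nodes for recording the bag in level save data and destroying it are disconnected, so an emptied bag stays in the world.
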(event `self.ReceiveBeginPlay`)

(event `self.InventorySystem.OnInventoryUpdate`
  (if (`/Game/Blueprints/Inventory/InventorySystem.isEmpty` (`self.InventorySystem`))
    (bind _asrs_player_controller (cast `/Game/Player/RS_PlayerController` (`GameplayStatics.GetPlayerController` 0)))
    (`/Game/Widgets/W_PlayerHud.HideContainer` (`/Game/Player/RS_PlayerController.HUD` _asrs_player_controller))))

(event `/Game/Blueprints/Inventory/BPI_InteractInterface.InteractWith`
  (params (PlayerC :type "/Game/Player/BP_Char Object Reference"))
  (bind _asrs_player_controller (cast `/Game/Player/RS_PlayerController` (`GameplayStatics.GetPlayerController` 0)))
  (`/Game/Widgets/W_PlayerHud.ShowContainer` (`/Game/Player/RS_PlayerController.HUD` _asrs_player_controller) (`self.InventorySystem`)))

(fn `LookAt`
  (returns (Message :type Text))
  (return ""))

(fn `UserConstructionScript`
  (`parent.UserConstructionScript`))