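; An item data component, apparently for inventory pickups, that sets its owning actor to replicate on BeginPlay.
; Its Interactwith event is empty, and LookAt returns an empty string.
; Disconnected pickup logic would add the item's row name and quantity to the player's InventorySystem and destroy the owner on success, but it never runs.
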(event `self.ReceiveBeginPlay`
  (`Actor.SetReplicates` (`self.GetOwner`) true))

(event `/Game/Blueprints/Inventory/BPI_InteractInterface.InteractWith`
  (params (PlayerC :type "/Game/Player/BP_Char Object Reference")))

(fn `LookAt`
  (returns (Message :type Text))
  (return ""))