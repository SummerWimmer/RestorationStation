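; Inventory component that lets its connected actor pick up, stack, consume and drop A_MasterItem items.
; The interact input tries items overlapping the actor's sphere, destroying the first one successfully added.
; Adding tops up matching stacks by name before appending a slot within the slot limit.
; Removal clears or decrements a slot, respawns unconsumed items at the actor, and, like pickup, fires OnUpdateInv.
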(event `EnhancedInput|/Game/Player/Input/Actions/IA_Interact`
  (params (ActionValue :type Boolean) (ElapsedSeconds :type "Float (double-precision)") (TriggeredSeconds :type "Float (double-precision)") (InputAction :type "InputAction Object Reference" :default "/Game/Player/Input/Actions/IA_Interact.IA_Interact"))
  (:`Completed`
    (for _array_element (`PrimitiveComponent.GetOverlappingActors` (`/Game/Player/BP_Char.Sphere` (`self.ConnectedActor`)) "/Game/Blueprints/Inventory/A_MasterItem.A_MasterItem_C")
      (bind _added_ (`self.TryAddItem` _array_element))
      (if _added_
        (`self.OnUpdateInv`)
        (`Actor.K2_DestroyActor` _array_element)
        (break)))))

(event `DropItem`
  (params (Quantity :type Integer) (InvIndex :type Integer))
  (bind _itemdata (break `/Game/Blueprints/Inventory/AC_InventorySlotStruct` (`|GetArrayItem` (`self.Inventory`) InvIndex)))
  (bind _returnvalue (`|SpawnActorFromClass` (`.class_23_C452E3B649ECEF64BC376381E16C2EC9` (break `/Game/Blueprints/Inventory/AC_ItemStruc` _itemdata)) (`Actor.GetTransform` (`self.ConnectedActor`)) "AlwaysSpawn" "MultiplyWithRoot" null null))
  (bind _output_get (set `/Game/Blueprints/Inventory/A_MasterItem.ItemData` _itemdata _returnvalue))
  (setmembers `/Game/Blueprints/Inventory/AC_ItemStruc` :`StructRef` _output_get :`Amount` Quantity))

(fn `AddItemAmountToInv`
  (params (Item :type "/Game/Blueprints/Inventory/AC_ItemStruc Structure") (amount :type Integer))
  (returns (ItemAdded :type Boolean))
  (bind (_name _description _catagory _value _amount _stacksize _texture _class) (break `/Game/Blueprints/Inventory/AC_ItemStruc` Item))
  (if (< (`KismetArrayLibrary.Array_Length` (`self.Inventory`)) (`self.InvSlotLimit`))
    (`KismetArrayLibrary.Array_Add` (`self.Inventory`) (make `/Game/Blueprints/Inventory/AC_InventorySlotStruct` (make `/Game/Blueprints/Inventory/AC_ItemStruc` _name _description _catagory _value amount _stacksize _texture _class) true))
    (return true)
    (else
      (return false))))

(fn `AddItemToInv`
  (params (Item :type "/Game/Blueprints/Inventory/AC_ItemStruc Structure"))
  (returns (ItemAdded :type Boolean))
  (if (< (`KismetArrayLibrary.Array_Length` (`self.Inventory`)) (`self.InvSlotLimit`))
    (`KismetArrayLibrary.Array_Add` (`self.Inventory`) (make `/Game/Blueprints/Inventory/AC_InventorySlotStruct` Item true))
    (return true)
    (else
      (return false))))

(fn `AddToStack`
  (params (Index :type Integer) (Amount :type Integer))
  (returns (exess :type Integer) (AllFit :type Boolean))
  (bind _output (`|GetArrayItem` (`self.Inventory`) Index))
  (bind _itemdata (break `/Game/Blueprints/Inventory/AC_InventorySlotStruct` _output))
  (bind ((`Amount_13_4D41187841EA78F19ACABE8C6AD216D1` _amount) (`StackSize_16_DC8B6A8D4A09FA382FDBC580BF107F3A` _stacksize)) (break `/Game/Blueprints/Inventory/AC_ItemStruc` _itemdata))
  (bind _returnvalue (+ (`local.Amount`) _amount))
  (if (> _returnvalue _stacksize)
    (bind _structout (setmembers `/Game/Blueprints/Inventory/AC_ItemStruc` :`StructRef` _itemdata :`Amount` _stacksize))
    (setmembers `/Game/Blueprints/Inventory/AC_InventorySlotStruct` :`StructRef` _output :`ItemData` _structout)
    (return (- _stacksize _returnvalue) false)
    (else
      (bind _structout_2 (setmembers `/Game/Blueprints/Inventory/AC_ItemStruc` :`StructRef` _itemdata :`Amount` _returnvalue))
      (setmembers `/Game/Blueprints/Inventory/AC_InventorySlotStruct` :`StructRef` _output :`ItemData` _structout_2)
      (return 0 true))))

(fn `FillableStacks`
  (params (Item :type "/Game/Blueprints/Inventory/AC_ItemStruc Structure"))
  (returns (InvIndexs :type "Array of Integer"))
  (locals (LOCAL_Index :type "Array of Integer"))
  (for (_array_element _array_index) (`self.Inventory`)
    (bind (_name _description _catagory _value _amount _stacksize) (break `/Game/Blueprints/Inventory/AC_ItemStruc` (break `/Game/Blueprints/Inventory/AC_InventorySlotStruct` _array_element)))
    (if (`KismetStringLibrary.EqualEqual_StrStr` _name (`.Name_2_3BFA498A46F6E38BF9865E99AD244CC4` (break `/Game/Blueprints/Inventory/AC_ItemStruc` Item)))
      (if (< _amount _stacksize)
        (`KismetArrayLibrary.Array_Add` (`local.LOCAL_Index`) _array_index))))
  (return (`local.LOCAL_Index`)))

(fn `IsSlotEmpty`
  (returns (SlotEmpty :type Boolean))
  (return (`.IsOccupied_5_C4DBFB7545E92A74A8D8DC9502C32E10` (break `/Game/Blueprints/Inventory/AC_InventorySlotStruct` (`|GetArrayItem` (`self.Inventory`))))))

(fn `RemoveFromInv`
  (params (Index :type Integer) (RemoveWholeStack :type Boolean) (IsConsumed :type Boolean))
  (locals (LOCAL_Quantity :type Integer))
  (bind _output_itemdata (break `/Game/Blueprints/Inventory/AC_InventorySlotStruct` (`|GetArrayItem` (`self.Inventory`) Index)))
  (bind _itemdata (break `/Game/Blueprints/Inventory/AC_InventorySlotStruct` (`|GetArrayItem` (`self.Inventory`) (`local.Index`))))
  (set `local.LOCAL_Quantity` (`.Amount_13_4D41187841EA78F19ACABE8C6AD216D1` (break `/Game/Blueprints/Inventory/AC_ItemStruc` _output_itemdata)))
  (`|ExecutionSequence`
    (:`then_0`
      (if (or (`local.RemoveWholeStack`) (< (`local.LOCAL_Quantity`) 2))
        (if (not (`local.IsConsumed`))
          (`self.DropItem` (`local.LOCAL_Quantity`) (`local.Index`)))
        (`KismetArrayLibrary.Array_Set` (`self.Inventory`) (`local.Index`))
        (else
          (setmembers `/Game/Blueprints/Inventory/AC_ItemStruc` :`StructRef` _itemdata :`Amount` (- (`.Amount_13_4D41187841EA78F19ACABE8C6AD216D1` (break `/Game/Blueprints/Inventory/AC_ItemStruc` _itemdata)) 1))
          (if (not (`local.IsConsumed`))
            (`self.DropItem` 1 (`local.Index`))))))
    (:`then_1`
      (`self.OnUpdateInv`))))

(fn `TryAddItem`
  (params (HitActor :type "Actor Object Reference"))
  (returns (`Added?` :type Boolean))
  (locals (CurrentItem :type "/Game/Blueprints/Inventory/AC_ItemStruc Structure") (LOCAL_AddedAll :type Boolean :default false) (LOCAL_Exess :type Integer :default 0))
  (bind _asa_master_item (cast `/Game/Blueprints/Inventory/A_MasterItem` HitActor)
    (:`then`
      (bind _output_get (set `local.CurrentItem` (`/Game/Blueprints/Inventory/A_MasterItem.ItemData` _asa_master_item)))
      (bind _invindexs (`self.FillableStacks` _output_get))
      (if (> (`KismetArrayLibrary.Array_Length` _invindexs) 0)
        (set `local.LOCAL_Exess` (`.Amount_13_4D41187841EA78F19ACABE8C6AD216D1` (break `/Game/Blueprints/Inventory/AC_ItemStruc` _output_get)))
        (for _array_element _invindexs
          (bind (_exess _allfit) (`self.AddToStack` _array_element (`local.LOCAL_Exess`)))
          (set `local.LOCAL_Exess` _exess)
          (set `local.LOCAL_AddedAll` _allfit))
        (if (`local.LOCAL_AddedAll`)
          (return true)
          (else
            (bind _itemadded (`self.AddItemAmountToInv` (`local.CurrentItem`) (`local.LOCAL_Exess`)))
            (return _itemadded)))
        (elif (< (`KismetArrayLibrary.Array_Length` (`self.Inventory`)) (`self.InvSlotLimit`))
          (bind _itemadded_2 (`self.AddItemToInv` (`local.CurrentItem`)))
          (return _itemadded_2)
          (else
            (set `local.CurrentItem` (struct))
            (return false)))))
    (:`CastFailed`
      (set `local.CurrentItem` (struct))
      (return false))))